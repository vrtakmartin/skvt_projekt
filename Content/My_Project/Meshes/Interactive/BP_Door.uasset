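; Interactive door that the player opens and closes with E while inside its trigger box, which also shows a prompt widget.
; The OpenDoor timeline plays or reverses to lerp the door mesh and widget yaw between 0 and 90 degrees.
; Flags track the open state and block input until the timeline finishes.
; BeginPlay hides the widget and runs the close branch to initialize the state.
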(event `self.SM_Door_A.OnBeginCursorOver`
  (params (TouchedComponent :type "PrimitiveComponent Object Reference")))

(event `self.Box.OnComponentBeginOverlap`
  (params (OverlappedComponent :type "PrimitiveComponent Object Reference") (OtherActor :type "Actor Object Reference") (OtherComp :type "PrimitiveComponent Object Reference") (OtherBodyIndex :type Integer) (bFromSweep :type Boolean) (SweepResult :type "HitResult Structure (by ref)"))
  ; Character is inside
  (`self.EnableInput` (`GameplayStatics.GetPlayerController` 0))
  (`SceneComponent.SetVisibility` (`self.Widget1`) true false))

(event `self.Box.OnComponentEndOverlap`
  (params (OverlappedComponent :type "PrimitiveComponent Object Reference") (OtherActor :type "Actor Object Reference") (OtherComp :type "PrimitiveComponent Object Reference") (OtherBodyIndex :type Integer))
  ; Character is inside
  (`self.DisableInput` (`GameplayStatics.GetPlayerController` 0))
  (`SceneComponent.SetVisibility` (`self.Widget1`) false false))

(event `Key|E`
  (params (Key :type "Key Structure"))
  (:`Pressed`
    (if (`self.IsTimeLineFinished`)
      (set `self.IsTimeLineFinished` false)
      (if (`self.IsDoorOpen`)
        (if (`self.IsDoorOpen`) :!label _label
          (set `self.IsDoorOpen` false)
          (bind (_direction _chestrotation) (`Timeline|OpenDoor` :!via `ReverseFromEnd` :!label _label_2)
            (:`Update`
              (bind _returnvalue (`KismetMathLibrary.Lerp` 0.0 90.0 _chestrotation))
              (`SceneComponent.K2_SetRelativeRotation` (`self.SM_Door_A`) (`KismetMathLibrary.MakeRotator` 0.0 0.0 _returnvalue) false false)
              (`SceneComponent.K2_SetRelativeRotation` (`self.Widget1`) (`KismetMathLibrary.MakeRotator` 0.0 0.0 _returnvalue) false false))
            (:`Finished`
              (set `self.IsTimeLineFinished` true :!label _label_3)))
          (else
            (goto _label_3)))
        (else
          (set `self.IsDoorOpen` true)
          (goto _label_2))))))

(event `self.ReceiveBeginPlay`
  (`SceneComponent.SetVisibility` (`self.Widget1`) false false)
  (goto _label))

(event `self.ReceiveTick`
  (params (DeltaSeconds :type "Float (single-precision)")))

(fn `UserConstructionScript`)