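; Interactive fire-and-smoke actor that the player toggles with E while inside its trigger box.
; Box overlap enables or disables player input and shows or hides a prompt widget, without filtering the overlapping actor.
; E drives a FlipFlop that switches the Niagara effect and point light together.
; Tick sends Ultra Dynamic Weather wind intensity and direction to Niagara, though both variable names are blank.
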(event `self.Box.OnComponentBeginOverlap`
  (params (OverlappedComponent :type "PrimitiveComponent Object Reference") (OtherActor :type "Actor Object Reference") (OtherComp :type "PrimitiveComponent Object Reference") (OtherBodyIndex :type Integer) (bFromSweep :type Boolean) (SweepResult :type "HitResult Structure (by ref)"))
  ; Character is inside
  (`self.EnableInput` (`GameplayStatics.GetPlayerController` 0))
  (`SceneComponent.SetVisibility` (`self.Widget1`) true false))

(event `self.Box.OnComponentEndOverlap`
  (params (OverlappedComponent :type "PrimitiveComponent Object Reference") (OtherActor :type "Actor Object Reference") (OtherComp :type "PrimitiveComponent Object Reference") (OtherBodyIndex :type Integer))
  ; Character is inside
  (`self.DisableInput` (`GameplayStatics.GetPlayerController` 0))
  (`SceneComponent.SetVisibility` (`self.Widget1`) false false))

(event `self.ReceiveTick`
  (params (DeltaSeconds :type "Float (single-precision)"))
  (`NiagaraComponent.SetNiagaraVariableFloat` (`self.NS_FireSmoke`) "" (`/Game/UltraDynamicSky/Blueprints/Functions/UltraDynamicWeather_Functions.Get Wind Intensity · 𝖴𝖣𝖶`))
  (`NiagaraComponent.SetNiagaraVariableVec3` (`self.NS_FireSmoke`) "" (`/Game/UltraDynamicSky/Blueprints/Functions/UltraDynamicWeather_Functions.Get Wind Direction Vector · 𝖴𝖣𝖶`)))

(event `self.ReceiveBeginPlay`
  (`SceneComponent.SetVisibility` (`self.Widget1`) false false)
  ; Vypnut na zaciatku
  (if false
    (`ActorComponent.SetActive` (`self.NS_FireSmoke`) (stale `Key|E` _isa) false :!label _label)
    (`SceneComponent.SetVisibility` (`self.PointLight`) (stale `Key|E` _isa) false)))

(event `Key|E`
  (params (Key :type "Key Structure"))
  (:`Pressed`
    (bind _isa (`/Engine/EditorBlueprintResources/StandardMacros.FlipFlop`)
      (:`A`
        (goto _label))
      (:`B`
        (goto _label)))))

(fn `UserConstructionScript`)